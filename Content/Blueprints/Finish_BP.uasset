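; Finish line actor for boat races that counts laps and signals when a player completes the race.
; On BeginPlay it gathers all Checkpoint actors to know how many exist.
; Box overlaps fire RuleComplete with the player's controller number if the boat can end.
; Otherwise, a boat past every checkpoint advances a lap, resets checkpoints, fires FinishLine and, under GM_Trial, stores lap times in the TrialManager.
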(event `self.ReceiveBeginPlay`
  (`self.Init`))

(event `Init`
  ;[1 1 1] Init
  (bind _outactors (`GameplayStatics.GetAllActorsOfClass` "/Game/Blueprints/Checkpoint.Checkpoint_C"))
  (set `self.Checkpoints` _outactors))

(event `self.Box.OnComponentBeginOverlap`
  (params (OverlappedComponent :type "PrimitiveComponent Object Reference") (OtherActor :type "Actor Object Reference") (OtherComp :type "PrimitiveComponent Object Reference") (OtherBodyIndex :type Integer) (bFromSweep :type Boolean) (SweepResult :type "HitResult Structure (by ref)"))
  ;[1 1 1] BeginOverlap
  (bind _asbase_boat_pawn (cast `/Game/Blueprints/BoatPawns/BaseBoat_Pawn` OtherActor))
  (if (`/Game/Blueprints/BoatPawns/BaseBoat_Pawn.canEnd?` _asbase_boat_pawn)
    (bind _asboat_pc (cast `/Game/Blueprints/Boat_PC` (`Pawn.GetController` _asbase_boat_pawn)))
    (`self.RuleComplete` (+ (`GameplayStatics.GetPlayerControllerID` _asboat_pc) 1))
    (elif (== (`KismetArrayLibrary.Array_LastIndex` (`self.Checkpoints`)) (- (`/Game/Blueprints/BoatPawns/BaseBoat_Pawn.CurrentCheckpoint` _asbase_boat_pawn) 1))
      (bind _returnvalue (+ (`/Game/Blueprints/BoatPawns/BaseBoat_Pawn.CurrentLap` _asbase_boat_pawn) 1))
      (set `/Game/Blueprints/BoatPawns/BaseBoat_Pawn.CurrentLap` _returnvalue _asbase_boat_pawn)
      (set `/Game/Blueprints/BoatPawns/BaseBoat_Pawn.CurrentCheckpoint` 0 _asbase_boat_pawn)
      (`self.FinishLine`)
      (bind _asgm_trial (cast `/Game/Blueprints/GameModes/GM_Trial` (`GameplayStatics.GetGameMode`)))
      (switch `int` _returnvalue
        (:`1`
          (bind _trialmanager (`/Game/Blueprints/GameModes/GM_Trial.TrialManager` _asgm_trial))
          (bind _timercount (`/Game/Blueprints/Trial_Manager.TimerCount` _trialmanager))
          (set `/Game/Blueprints/Trial_Manager.Lap1Time` _timercount _trialmanager))
        (:`2`
          (set `/Game/Blueprints/Trial_Manager.Lap2Time` _timercount _trialmanager))
        (:`3`
          (set `/Game/Blueprints/Trial_Manager.Lap3Time` _timercount _trialmanager))))))

(fn `UserConstructionScript`)