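; PointsManager tracks Character1Points and displays a points HUD for the game.
; On BeginPlay it creates the PointsHUDUI widget, passes itself to it, then sets the points to GameStartPoints.
; Its LogPoints event binds a penalty handler to every BaseObstacle_BP actor's minus-log-points event.
; That handler assigns LogMinus10Points to Character1Points when a log is hit.
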(event `self.ReceiveBeginPlay`
  (bind _returnvalue (`|CreateWidget` "/Game/Blueprints/PointsHUDUI.PointsHUDUI_C"))
  (bind _output_get (set `self.PointsREF` _returnvalue))
  (`UserWidget.AddToViewport` _output_get 0)
  (`/Game/Blueprints/PointsHUDUI.InitPointsText` _output_get self)
  (set `self.Character1Points` (`self.GameStartPoints`)))

(event `LogPoints`
  (bind _outactors (`GameplayStatics.GetAllActorsOfClass` "/Game/Blueprints/BaseObstacle_BP.BaseObstacle_BP_C"))
  (bind _output_get (set `self.Out Actors` _outactors))
  (for _array_element _output_get
    (add `/Game/Blueprints/BaseObstacle_BP.MinusLogPoints` _array_element (delegate `TakeawayPointsForHittingLog`))))

(event `TakeawayPointsForHittingLog`
  (set `self.Character1Points` (`self.LogMinus10Points`)))

(fn `UserConstructionScript`)