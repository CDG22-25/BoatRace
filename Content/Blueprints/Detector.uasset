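; Detector is a downward surface probe that flags whether movement is allowed, based on water beneath it.
; While enabled, it line-traces on the Visibility channel every Tick from its world location straight down by a configurable Distance.
; CanMove becomes true when the hit actor carries the Water tag, and false on a miss or any other valid actor.
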(event `self.ReceiveTick`
  (params (DeltaSeconds :type "Float (single-precision)"))
  (bind _returnvalue (`self.K2_GetComponentLocation` self))
  (if (`self.Enable`)
    (bind (_outhit _returnvalue_2) (`KismetSystemLibrary.LineTraceSingle` _returnvalue (- _returnvalue (`KismetMathLibrary.MakeVector` 0.0 0.0 (`self.Distance`))) "TraceTypeQuery1"))
    (if _returnvalue_2
      (`/Engine/EditorBlueprintResources/StandardMacros.IsValid` (`.HitActor` (`GameplayStatics.BreakHitResult` _outhit))
        (:`Is Valid`
          (if (`KismetArrayLibrary.Array_Contains` (`Actor.Tags` (`.HitActor` (`GameplayStatics.BreakHitResult` _outhit))) "Water")
            (set `self.CanMove` true)
            (else
              (set `self.CanMove` false :!label _label)))))
      (else
        (goto _label)))))