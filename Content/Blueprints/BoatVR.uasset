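; VR player boat driven by physics, with four hover components, automatic forward thrust, a jump and twin cannons.
; A looping timer pushes the mesh forward, while input adds thrust and yaw torque that flips when moving backwards.
; Each cannon spawns a projectile and applies recoil impulse at its location, with its own cooldown.
; A height check on Tick briefly disables input to curb flying, and BeginPlay sets eye-level tracking origin.
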(event `self.ReceiveTick`
  (params (DeltaSeconds :type "Float (single-precision)"))
  (bind (_returnvalue_x _returnvalue_y _returnvalue_z) (`KismetMathLibrary.BreakVector` (`self.K2_GetActorLocation`)))
  ;[1 1 1] Flying Fix
  (if (> _returnvalue_z 300.0)
    (`self.DisableInput` null)
    (`KismetSystemLibrary.Delay` 2.0)
    (`self.EnableInput` null)))

(event `self.ReceiveBeginPlay`
  (bind _staticmesh (`self.StaticMesh`))
  (`|ExecutionSequence`
    (:`then_0`
      (`/Game/Blueprints/HoverComponent_SC.InitComponent` (`self.HoverComponent_SC`) _staticmesh)
      (`/Game/Blueprints/HoverComponent_SC.InitComponent` (`self.HoverComponent_SC1`) _staticmesh)
      (`/Game/Blueprints/HoverComponent_SC.InitComponent` (`self.HoverComponent_SC2`) _staticmesh)
      (`/Game/Blueprints/HoverComponent_SC.InitComponent` (`self.HoverComponent_SC3`) _staticmesh)
      (`self.AutoMove`))
    (:`then_1`
      (`HeadMountedDisplayFunctionLibrary.SetTrackingOrigin` "Eye")
      (`SceneComponent.K2_SetRelativeLocation` (`self.VRCameraRoot`) (`self.CameraHeight`) false false))))

(event `AutoMove`
  ;[1 1 1] Auto Move
  (bind _returnvalue (`KismetSystemLibrary.K2_SetTimerDelegate` (delegate `MoveTimer`) 0.1 true))
  (set `self.MoveHandle` _returnvalue))

(event `InputAxis|MoveForward`
  (params (AxisValue :type "Float (single-precision)"))
  ;[1 1 1] Movement
  (`PrimitiveComponent.AddForce` (`self.StaticMesh`) (* (* (`self.GetActorForwardVector`) (`self.ForwardSpeed`)) AxisValue) "None" true))

(event `InputAction|Jump`
  (params (Key :type "Key Structure"))
  ;[1 1 1] Movement
  (:`Pressed`
    (if (`self.canJump`)
      (`PrimitiveComponent.AddForce` (`self.StaticMesh`) (* (`self.GetActorUpVector`) (`self.JumpStrength`)) "None" true)
      (set `self.canJump` false)
      (`KismetSystemLibrary.Delay` (`self.JumpDelay`))
      (set `self.canJump` true))))

(event `MoveTimer`
  ;[1 1 1] Auto Move
  (`PrimitiveComponent.AddForce` (`self.StaticMesh`) (* (`self.GetActorForwardVector`) 7000.0) "None" true))

(event `InputAxis|MoveRight`
  (params (AxisValue :type "Float (single-precision)"))
  ;[1 1 1] Movement
  (bind _returnvalue (`PrimitiveComponent.GetPhysicsLinearVelocity` (`self.StaticMesh`) "None"))
  (`PrimitiveComponent.AddTorqueInDegrees` (`self.StaticMesh`) (`KismetMathLibrary.MakeVector` 0.0 0.0 (* (`KismetMathLibrary.SelectFloat` 1.0 -1.0 (> (`KismetMathLibrary.Dot_VectorVector` _returnvalue (`self.GetActorForwardVector`)) 0.0)) (* AxisValue (`self.TurningSpeed`)))) "None" true))

(event `InputAction|FireR`
  (params (Key :type "Key Structure"))
  (bind _rcannon (`self.RCannon`))
  (bind (_returnvalue_location _returnvalue_rotation) (`KismetMathLibrary.BreakTransform` (`SceneComponent.K2_GetComponentToWorld` _rcannon)))
  ;[1 1 1] Fire
  (:`Pressed`
    (if (`self.canBeFiredR`)
      (`PrimitiveComponent.AddImpulseAtLocation` (`self.StaticMesh`) (* (`SceneComponent.GetForwardVector` _rcannon) -500000.0) (`SceneComponent.K2_GetComponentLocation` _rcannon) "None")
      (`|SpawnActorFromClass` (`self.Projectile`) (`KismetMathLibrary.MakeTransform` _returnvalue_location _returnvalue_rotation (`self.ProjectileSize`)) "AdjustIfPossibleButAlwaysSpawn" "OverrideRootScale" null null)
      (set `self.canBeFiredR` false)
      (`KismetSystemLibrary.Delay` (`self.FireDelay`))
      (set `self.canBeFiredR` true))))

(event `InputAction|FireL`
  (params (Key :type "Key Structure"))
  (bind _lcannon (`self.LCannon`))
  (bind (_returnvalue_location _returnvalue_rotation) (`KismetMathLibrary.BreakTransform` (`SceneComponent.K2_GetComponentToWorld` _lcannon)))
  ;[1 1 1] Fire
  (:`Pressed`
    (if (`self.canBeFiredL`)
      (`PrimitiveComponent.AddImpulseAtLocation` (`self.StaticMesh`) (* (`SceneComponent.GetForwardVector` _lcannon) -500000.0) (`SceneComponent.K2_GetComponentLocation` _lcannon) "None")
      (`|SpawnActorFromClass` (`self.Projectile`) (`KismetMathLibrary.MakeTransform` _returnvalue_location _returnvalue_rotation (`self.ProjectileSize`)) "AdjustIfPossibleButAlwaysSpawn" "OverrideRootScale" null null)
      (set `self.canBeFiredL` false)
      (`KismetSystemLibrary.Delay` (`self.FireDelay`))
      (set `self.canBeFiredL` true))))

(fn `UserConstructionScript`)