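; SelectManager coordinates boat selection for multiple players on a player select screen.
; Init caches every player controller, ordered by player index, along with all BoatSelector actors in the level.
; NextBoat and PrevBoat match the calling controller's array index to a selector's PlayerIndex and cycle that selector's boat forward or back.
; The resulting boat type then goes to that PlayerSelect_PC through SetBoatMessage.
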(event `Init`
  (params (UI :type "PlayerController Object Reference"))
  ;[1 1 1] Init
  (`self.GetControllers`)
  (`self.GetBoatSelectors`))

(event `NextBoat`
  (params (Controller :type "PlayerController Object Reference"))
  (bind _asplayer_select_pc (cast `/Game/Blueprints/PlayerSelect_PC` Controller :!pure true))
  ;[1 1 1] Change Boat
  (for _array_element (`self.BoatSelectors`)
    (if (== (`/Game/Blueprints/BoatSelector.playerIndex` _array_element) (`KismetArrayLibrary.Array_Find` (`self.Controllers`) _asplayer_select_pc))
      (`/Game/Blueprints/BoatSelector.UpdateBoat` _array_element true)
      (break)))
  (message `/Game/Blueprints/I_Boat.SetBoat` _asplayer_select_pc (`/Game/Blueprints/BoatSelector.BoatType` _array_element)))

(event `PrevBoat`
  (params (Controller :type "PlayerController Object Reference"))
  (bind _asplayer_select_pc (cast `/Game/Blueprints/PlayerSelect_PC` Controller :!pure true))
  ;[1 1 1] Change Boat
  (for _array_element (`self.BoatSelectors`)
    (if (== (`/Game/Blueprints/BoatSelector.playerIndex` _array_element) (`KismetArrayLibrary.Array_Find` (`self.Controllers`) _asplayer_select_pc))
      (`/Game/Blueprints/BoatSelector.UpdateBoat` _array_element false)
      (break)))
  (message `/Game/Blueprints/I_Boat.SetBoat` _asplayer_select_pc (`/Game/Blueprints/BoatSelector.BoatType` _array_element)))

(fn `GetBoatSelectors`
  (bind _outactors (`GameplayStatics.GetAllActorsOfClass` "/Game/Blueprints/BoatSelector.BoatSelector_C"))
  (for _array_element _outactors
    (`KismetArrayLibrary.Array_AddUnique` (`self.BoatSelectors`) _array_element)))

(fn `GetControllers`
  (bind _outactors (`GameplayStatics.GetAllActorsOfClass` "/Script/Engine.PlayerController"))
  (for _index (range (+ (`KismetArrayLibrary.Array_LastIndex` _outactors) 1))
    (`KismetArrayLibrary.Array_AddUnique` (`self.Controllers`) (`GameplayStatics.GetPlayerController` _index))))

(fn `UserConstructionScript`)