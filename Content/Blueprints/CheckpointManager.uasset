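; CheckpointManager gathers race checkpoints and boats, apparently as groundwork for tracking boat positions.
; BeginPlay fills CheckpointArray and BoatArray using GetAllActorsOfClass.
; PositionTick, which nothing in this graph calls, starts a fast looping timer stored in PositionHandle.
; The timer loops over the boats but does nothing yet, leaving an unconnected CurrentCheckpoint read as unfinished position logic.
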(event `self.ReceiveBeginPlay`
  (bind _outactors (`GameplayStatics.GetAllActorsOfClass` "/Game/Blueprints/Checkpoint.Checkpoint_C"))
  (set `self.CheckpointArray` _outactors)
  (bind _outactors_2 (`GameplayStatics.GetAllActorsOfClass` "/Game/Blueprints/BoatPawns/BaseBoat_Pawn.BaseBoat_Pawn_C"))
  (set `self.BoatArray` _outactors_2))

(event `PositionTick`
  (bind _returnvalue (`KismetSystemLibrary.K2_SetTimerDelegate` (delegate `Timer`) 0.1 true))
  (set `self.PositionHandle` _returnvalue))

(event `Timer`
  (for _array_element (`self.BoatArray`)
    _))

(fn `UserConstructionScript`)