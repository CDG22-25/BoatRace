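; BoatSpawner is a placeable spawner that creates a boat of a configurable class and can hand it to a player.
; Shortly after BeginPlay it spawns BoatType at its own location and rotation with BoatScale, ignoring collisions.
; If PlayerEnabled is set and the controller at PlayerIndex is valid, that controller possesses the boat and its name is printed.
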(event `self.ReceiveBeginPlay`
  (bind (_returnvalue_location _returnvalue_rotation) (`KismetMathLibrary.BreakTransform` (`self.GetTransform`)))
  (bind _returnvalue (`GameplayStatics.GetPlayerController` (`self.Player Index`)))
  (`KismetSystemLibrary.Delay` 0.1)
  (bind _returnvalue_2 (`|SpawnActorFromClass` (`self.BoatType`) (`KismetMathLibrary.MakeTransform` _returnvalue_location _returnvalue_rotation (`self.BoatScale`)) "AlwaysSpawn" "OverrideRootScale" null null))
  (if (`self.playerEnabled?`)
    (`/Engine/EditorBlueprintResources/StandardMacros.IsValid` _returnvalue
      (:`Is Valid`
        (`Controller.Possess` _returnvalue _returnvalue_2)
        (`KismetSystemLibrary.PrintString` (`KismetSystemLibrary.GetDisplayName` _returnvalue))))))

(fn `UserConstructionScript`)