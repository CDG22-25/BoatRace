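; SelectManager runs boat selection on the player select screen, linking player controllers to the level's BoatSelector actors.
; Init stores the UI, gathers selectors, takes controllers from GM_PlayerSelect, and for one player hides the index 1 selector and clears a UI text.
; NextBoat and PrevBoat match the controller's array index to a selector's PlayerIndex, cycle its boat, then send the BoatType to that controller.
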(event `Init`
  (params (UI :type "/Game/UI/Selection_UI Object Reference") (PlayerControllers :type "Array of PlayerController Object Reference") (`Number of Players` :type Integer))
  ;[1 1 1] Init
  (set `self.Controllers` PlayerControllers)
  (set `self.UI` UI)
  (`self.GetBoatSelectors`)
  (`self.GetControllers`)
  (`self.CorrectPlayers` `Number of Players`))

(event `NextBoat`
  (params (Controller :type "PlayerController Object Reference"))
  (bind _asplayer_select_pc (cast `/Game/Blueprints/PlayerSelect_PC` Controller :!pure true))
  ;[1 1 1] Change Boat
  (for _array_element (`self.BoatSelectors`)
    (if (== (`/Game/Blueprints/BoatSelector.playerIndex` _array_element) (`KismetArrayLibrary.Array_Find` (`self.Controllers`) _asplayer_select_pc))
      (`/Game/Blueprints/BoatSelector.UpdateBoat` _array_element true)
      (break)))
  (message `/Game/Blueprints/I_Boat.SetBoat` _asplayer_select_pc (`/Game/Blueprints/BoatSelector.BoatType` _array_element)))

(event `PrevBoat`
  (params (Controller :type "PlayerController Object Reference"))
  (bind _asplayer_select_pc (cast `/Game/Blueprints/PlayerSelect_PC` Controller :!pure true))
  ;[1 1 1] Change Boat
  (for _array_element (`self.BoatSelectors`)
    (if (== (`/Game/Blueprints/BoatSelector.playerIndex` _array_element) (`KismetArrayLibrary.Array_Find` (`self.Controllers`) _asplayer_select_pc))
      (`/Game/Blueprints/BoatSelector.UpdateBoat` _array_element false)
      (break)))
  (message `/Game/Blueprints/I_Boat.SetBoat` _asplayer_select_pc (`/Game/Blueprints/BoatSelector.BoatType` _array_element)))

(fn `CorrectPlayers`
  (params (`Number of Players` :type Integer))
  (switch `int` `Number of Players`
    (:`1`
      (for _array_element (`self.BoatSelectors`)
        (if (== (`/Game/Blueprints/BoatSelector.playerIndex` _array_element) 1)
          (`self.SetActorHiddenInGame` _array_element true)))
      (`TextBlock.SetText` (`/Game/UI/Selection_UI.TextBlock` (`self.UI`)) ""))))

(fn `GetBoatSelectors`
  (bind _outactors (`GameplayStatics.GetAllActorsOfClass` "/Game/Blueprints/BoatSelector.BoatSelector_C"))
  (for _array_element _outactors
    (`KismetArrayLibrary.Array_AddUnique` (`self.BoatSelectors`) _array_element)))

(fn `GetControllers`
  (bind _asgm_player_select (cast `/Game/Blueprints/GameModes/GM_PlayerSelect` (`GameplayStatics.GetGameMode`)))
  (set `self.Controllers` (`/Game/Blueprints/GameModes/GM_PlayerSelect.PlayerControllers` _asgm_player_select)))

(fn `UserConstructionScript`)