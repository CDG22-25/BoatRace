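; Base boat pawn: a physics-driven hover boat, either player-controlled or moved along a spline as CPU when unpossessed.
; Four hover components support the mesh, while forces and torque drive steering, jumping and a timer-based forward push without throttle.
; Left and right cannons spawn projectiles with recoil and timeline cooldowns shown on widgets.
; Projectile hits add impulse, flash the mesh and briefly disable input; it also handles pause, reverse camera and post-game lockout.
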(event `self.ReceiveBeginPlay`
  (bind (_impactforce _knockback) (defaults `Object` (`self.Projectile`)))
  (bind _spline (`/Game/Blueprints/Spline_BP.Spline` (`self.splineReference`)))
  ;[1 1 1] Init
  (set `self.ImpactForce` _impactforce)
  (set `self.Kickback` _knockback)
  (`self.InitHoverComponents`)
  (`self.AutoMove`)
  (`self.SetProjectileWidgets`)
  (`KismetSystemLibrary.Delay` 0.2)
  (if (`self.isPossessed`)
    (set `self.canJump` true)
    (else
      (`/Engine/EditorBlueprintResources/StandardMacros.IsValid` (`self.splineReference`)
        (:`Is Valid`
          ;[1 1 1] CPU
          (bind (_direction _alpha) (`Timeline|SplineTimeline` :!via `PlayFromStart` :!label _label)
            (:`Update`
              (bind (_returnvalue_location _returnvalue_rotation) (`KismetMathLibrary.BreakTransform` (`SplineComponent.GetTransformAtDistanceAlongSpline` _spline (* _alpha (`SplineComponent.GetSplineLength` _spline)) "World" false)))
              (`self.K2_SetActorTransform` (`KismetMathLibrary.MakeTransform` _returnvalue_location _returnvalue_rotation (`SceneComponent.K2_GetComponentScale` (`self.StaticMesh`)))))))))))

(event `self.ReceiveHit`
  (params (MyComp :type "PrimitiveComponent Object Reference") (Other :type "Actor Object Reference") (OtherComp :type "PrimitiveComponent Object Reference") (bSelfMoved :type Boolean) (HitLocation :type "Vector Structure") (HitNormal :type "Vector Structure") (NormalImpulse :type "Vector Structure") (Hit :type "HitResult Structure (by ref)"))
  ;[1 1 1] Points System Damage
  (`GameplayStatics.ApplyDamage` Other 5.0))

(event `Init`
  ;[1 1 1] Init
)

(event `Continue`
  ;[1 1 1] CPU
  (goto _label))

(event `Damage`
  ;[1 1 1] CPU
  (goto _label :!via `Stop`))

(event `self.ReceiveTick`
  (params (DeltaSeconds :type "Float (single-precision)"))
  ;[1 1 1] Flying Fix
)

(event `InputAction|Reverse Camera`
  (params (Key :type "Key Structure"))
  (bind _springarm (`self.SpringArm`))
  ;[1 1 1] ReverseCam
  (:`Pressed`
    (`SceneComponent.K2_SetRelativeRotation` _springarm (struct :`Yaw` 180.0) false false))
  (:`Released`
    (`SceneComponent.K2_SetRelativeRotation` :`self` _springarm)))

(event `/Game/Blueprints/I_GameState.GameStateChanged`
  (params (newGameState :type "/Game/Blueprints/E_GameState Enum" :default "NewEnumerator0"))
  ;[1 1 1] Has Game Ended?
  (switch `/Game/Blueprints/E_GameState` newGameState
    (:`NewEnumerator3`
      (set `self.canBeFiredL` false)
      (set `self.canBeFiredR` false)
      (set `self.canJump` false)
      (set `self.canMove` false))))

(event `InputAxis|MoveForward`
  (params (AxisValue :type "Float (single-precision)"))
  ;[1 1 1] Movement
  (set `self.Axis Value` AxisValue)
  (if (`self.canMove`)
    (`PrimitiveComponent.AddForce` (`self.StaticMesh`) (* (* (`self.GetActorForwardVector`) (`self.ForwardSpeed`)) AxisValue) "None" true)
    (if (!= (`self.Axis Value`) 0.0)
      (set `self.Moving` true)
      (else
        (set `self.Moving` false)))))

(event `InputAction|Jump`
  (params (Key :type "Key Structure"))
  ;[1 1 1] Movement
  (:`Pressed`
    (if (`self.canJump`)
      (`PrimitiveComponent.AddForce` (`self.StaticMesh`) (* (`self.GetActorUpVector`) (`self.JumpStrength`)) "None" true)
      (set `self.canJump` false)
      (`KismetSystemLibrary.Delay` (`self.JumpDelay`))
      (set `self.canJump` true))))

(event `AutoMove`
  ;[1 1 1] Auto Move
  (bind _returnvalue (`KismetSystemLibrary.K2_SetTimerDelegate` (delegate `MoveTimer`) 0.1 true))
  (set `self.MoveHandle` _returnvalue))

(event `MoveTimer`
  ;[1 1 1] Auto Move
  (if (== (`self.Axis Value`) 0.0)
    (`PrimitiveComponent.AddForce` (`self.StaticMesh`) (* (`self.GetActorForwardVector`) 7000.0) "None" true)))

(event `InputAxis|MoveRight`
  (params (AxisValue :type "Float (single-precision)"))
  ;[1 1 1] Movement
  (if (`self.canMove`)
    (bind _returnvalue (`PrimitiveComponent.GetPhysicsLinearVelocity` (`self.StaticMesh`) "None"))
    (`PrimitiveComponent.AddTorqueInDegrees` (`self.StaticMesh`) (`KismetMathLibrary.MakeVector` 0.0 0.0 (* (`KismetMathLibrary.SelectFloat` 1.0 -1.0 (> (`KismetMathLibrary.Dot_VectorVector` _returnvalue (`self.GetActorForwardVector`)) 0.0)) (* AxisValue (`self.TurningSpeed`)))) "None" true)))

(event `InputAction|FireR`
  (params (Key :type "Key Structure"))
  (bind _rcannon (`self.RCannon`))
  (bind (_returnvalue_location _returnvalue_rotation) (`KismetMathLibrary.BreakTransform` (`SceneComponent.K2_GetComponentToWorld` _rcannon)))
  ;[1 1 1] Fire
  (:`Pressed`
    (if (`self.canBeFiredR`)
      (`PrimitiveComponent.AddImpulseAtLocation` (`self.StaticMesh`) (* (`SceneComponent.GetForwardVector` _rcannon) (`self.Kickback`)) (`SceneComponent.K2_GetComponentLocation` _rcannon) "None")
      (`|SpawnActorFromClass` (`self.Projectile`) (`KismetMathLibrary.MakeTransform` _returnvalue_location _returnvalue_rotation (`self.ProjectileSize`)) "AdjustIfPossibleButAlwaysSpawn" "OverrideRootScale" null null)
      (set `self.canBeFiredR` false)
      (`self.CoolDownR`))))

(event `InputAction|PauseGame` :paused true
  (params (Key :type "Key Structure"))
  (bind _returnvalue (`GameplayStatics.GetPlayerController` 0))
  ;[1 1 1] Pause Menu
  (:`Pressed`
    (if (`self.Is Game Paused?`)
      (set `self.Is Game Paused?` false)
      (`Widget.RemoveFromParent` (`self.PauseMenuREF`))
      (`GameplayStatics.SetGamePaused` false)
      (`WidgetBlueprintLibrary.SetInputMode_GameOnly` _returnvalue)
      (set `PlayerController.bShowMouseCursor` false _returnvalue)
      (else
        (set `self.Is Game Paused?` true)
        (bind _returnvalue_2 (`|CreateWidget` "/Game/EdwardsFile/UI/PauseMenu.PauseMenu_C" _returnvalue))
        (`UserWidget.AddToViewport` _returnvalue_2 0)
        (bind _output_get (set `self.PauseMenuREF` _returnvalue_2))
        (`UserWidget.AddToPlayerScreen` _output_get 0)
        (set `PlayerController.bShowMouseCursor` true _returnvalue)
        (`GameplayStatics.SetGamePaused` true)))))

(event `CoolDownR`
  ;[1 1 1] Cooldown Switch R
  (switch `/Game/Blueprints/BoatPawns/Cooldown_Enum` (`self.FireDelay`)
    (:`NewEnumerator0`
      (bind (_direction _percentage) (`Timeline|RCooldown1` :!via `PlayFromStart`)
        (:`Update`
          (`/Game/UI/ProjectileWidget.UpdateUI` (`self.RProjectileUI`) _percentage))
        (:`Finished`
          (set `self.canBeFiredR` true))))
    (:`NewEnumerator1`
      (bind (_direction_2 _percentage_2) (`Timeline|RCoolDown2` :!via `PlayFromStart`)
        (:`Update`
          (`/Game/UI/ProjectileWidget.UpdateUI` (`self.RProjectileUI`) _percentage_2))
        (:`Finished`
          (set `self.canBeFiredR` true))))
    (:`NewEnumerator2`
      (bind (_direction_3 _percentage_3) (`Timeline|RCoolDown5` :!via `PlayFromStart`)
        (:`Update`
          (`/Game/UI/ProjectileWidget.UpdateUI` (`self.RProjectileUI`) _percentage_3))
        (:`Finished`
          (set `self.canBeFiredR` true))))))

(event `InputAction|FireL`
  (params (Key :type "Key Structure"))
  (bind _lcannon (`self.LCannon`))
  (bind (_returnvalue_location _returnvalue_rotation) (`KismetMathLibrary.BreakTransform` (`SceneComponent.K2_GetComponentToWorld` _lcannon)))
  ;[1 1 1] Fire
  (:`Pressed`
    (if (`self.canBeFiredL`)
      (`PrimitiveComponent.AddImpulseAtLocation` (`self.StaticMesh`) (* (`SceneComponent.GetForwardVector` _lcannon) (`self.Kickback`)) (`SceneComponent.K2_GetComponentLocation` _lcannon) "None")
      (`|SpawnActorFromClass` (`self.Projectile`) (`KismetMathLibrary.MakeTransform` _returnvalue_location _returnvalue_rotation (`self.ProjectileSize`)) "AdjustIfPossibleButAlwaysSpawn" "OverrideRootScale" null null)
      (set `self.canBeFiredL` false)
      (`self.CoolDownL`))))

(event `self.StaticMesh.OnComponentHit`
  (params (HitComponent :type "PrimitiveComponent Object Reference") (OtherActor :type "Actor Object Reference") (OtherComp :type "PrimitiveComponent Object Reference") (NormalImpulse :type "Vector Structure") (Hit :type "HitResult Structure (by ref)"))
  (bind (_bblockinghit _binitialoverlap _time _distance _location _impactpoint _normal _impactnormal _physmat _hitactor) (`GameplayStatics.BreakHitResult` Hit))
  (bind _staticmesh (`self.StaticMesh`))
  ;[1 1 1] Damage
  (bind _asbase_projectile (castclass `/Game/Blueprints/Projectiles/Base_Projectile` (`GameplayStatics.GetObjectClass` _hitactor)))
  (bind _returnvalue (`GameplayStatics.GetActorOfClass` _asbase_projectile))
  (`PrimitiveComponent.AddImpulseAtLocation` (`self.StaticMesh`) (* (`self.GetActorForwardVector` _returnvalue) (`/Game/Blueprints/Projectiles/Base_Projectile.ImpactForce` _returnvalue)) _impactpoint "None")
  (`self.K2_DestroyActor` _returnvalue)
  (`self.DamageFlash`)
  (`|ExecutionSequence`
    (:`then_0`
      (bind _asboat_pc (cast `/Game/Blueprints/Boat_PC` (`self.GetController` self)))
      (`self.DisableInput` _asboat_pc)
      (`KismetSystemLibrary.Delay` (`self.DamageDuration`))
      (`self.EnableInput` null))
    (:`then_1`
      (`KismetSystemLibrary.Delay` (`self.DamageDuration`))
      (`KismetSystemLibrary.K2_ClearAndInvalidateTimerHandle` (`self.FlashTimerHandle`))
      (`SceneComponent.SetVisibility` _staticmesh true true)
      (cast `/Game/Blueprints/BoatPawns/Construction_Pawn` self)
      (`SceneComponent.SetVisibility` _staticmesh false false))))

(event `DamageFlash`
  ;[1 1 1] Flash
  (bind _returnvalue (`KismetSystemLibrary.K2_SetTimerDelegate` (delegate `Flash`) 0.1 true))
  (set `self.FlashTimerHandle` _returnvalue))

(event `CoolDownL`
  ;[1 1 1] CooldownL
  (switch `/Game/Blueprints/BoatPawns/Cooldown_Enum` (`self.FireDelay`)
    (:`NewEnumerator0`
      (bind (_direction _percentage) (`Timeline|LCooldown1` :!via `PlayFromStart`)
        (:`Update`
          (`/Game/UI/ProjectileWidget.UpdateUI` (`self.LProjectileUI`) _percentage))
        (:`Finished`
          (set `self.canBeFiredL` true))))
    (:`NewEnumerator1`
      (bind (_direction_2 _percentage_2) (`Timeline|LCoolDown2` :!via `PlayFromStart`)
        (:`Update`
          (`/Game/UI/ProjectileWidget.UpdateUI` (`self.LProjectileUI`) _percentage_2))
        (:`Finished`
          (set `self.canBeFiredL` true))))
    (:`NewEnumerator2`
      (bind (_direction_3 _percentage_3) (`Timeline|LCoolDown5` :!via `PlayFromStart`)
        (:`Update`
          (`/Game/UI/ProjectileWidget.UpdateUI` (`self.LProjectileUI`) _percentage_3))
        (:`Finished`
          (set `self.canBeFiredL` true))))))

(event `Flash`
  ;[1 1 1] Flash
  (`SceneComponent.ToggleVisibility` (`self.StaticMesh`) true))

(fn `InitHoverComponents`
  (bind _staticmesh (`self.StaticMesh`))
  (`/Game/Blueprints/HoverComponent_SC.InitComponent` (`self.HoverComponent_SC`) _staticmesh)
  (`/Game/Blueprints/HoverComponent_SC.InitComponent` (`self.HoverComponent_SC1`) _staticmesh)
  (`/Game/Blueprints/HoverComponent_SC.InitComponent` (`self.HoverComponent_SC2`) _staticmesh)
  (`/Game/Blueprints/HoverComponent_SC.InitComponent` (`self.HoverComponent_SC3`) _staticmesh))

(fn `SetProjectileWidgets`
  (bind _asprojectile_widget (cast `/Game/UI/ProjectileWidget` (`WidgetComponent.GetUserWidgetObject` (`self.RWidget`))))
  (set `self.RProjectileUI` _asprojectile_widget)
  (bind _asprojectile_widget_2 (cast `/Game/UI/ProjectileWidget` (`WidgetComponent.GetUserWidgetObject` (`self.LWidget`))))
  (set `self.LProjectileUI` _asprojectile_widget_2))

(fn `UserConstructionScript`)