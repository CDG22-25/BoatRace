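; DiggerBoat is a hovering physics boat pawn for a checkpoint race with cannon combat.
; Input drives force-based movement, jumping and two recoiling cannons with timeline cooldown widgets, while a timer pushes forward without throttle.
; Unpossessed boats follow a spline by timeline.
; Projectile hits add impulse, flash the mesh and briefly disable input or pause spline travel; skipping checkpoints teleports the boat back, and game end locks controls.
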(event `Continue`
  (bind _spline (`/Game/Blueprints/Spline_BP.Spline` (`self.splineReference`)))
  ;[1 1 1] CPU
  (bind (_direction _alpha) (`Timeline|SplineTimeline` :!label _label)
    (:`Update`
      (bind (_returnvalue_location _returnvalue_rotation) (`KismetMathLibrary.BreakTransform` (`SplineComponent.GetTransformAtDistanceAlongSpline` _spline (* _alpha (`SplineComponent.GetSplineLength` _spline)) "World" false)))
      (`self.K2_SetActorTransform` (`KismetMathLibrary.MakeTransform` _returnvalue_location _returnvalue_rotation (`SceneComponent.K2_GetComponentScale`))))))

(event `self.ReceiveBeginPlay`
  ;[1 1 1] Begin Play
  (`self.InitHoverComponents`)
  (`self.AutoMove`)
  (`self.SetProjectileWidgets`)
  (`KismetSystemLibrary.Delay` 0.2)
  (if (not (`self.isPossessed`))
    (`/Engine/EditorBlueprintResources/StandardMacros.IsValid` (`self.splineReference`)
      (:`Is Valid`
        (goto _label :!via `PlayFromStart`)))))

(event `Damage`
  ;[1 1 1] CPU
  (goto _label :!via `Stop`))

(event `self.ReceiveTick`
  (params (DeltaSeconds :type "Float (single-precision)"))
  (bind (_returnvalue_x _returnvalue_y _returnvalue_z) (`KismetMathLibrary.BreakVector` (`self.K2_GetActorLocation`)))
  ;[1 1 1] Flying Fix
  (`|ExecutionSequence`
    (:`then_0`
      (if (> _returnvalue_z 300.0)
        (set `self.canJump` false)
        (set `self.canMove` false)
        (`KismetSystemLibrary.Delay` 3.0)
        (set `self.canJump` true)
        (set `self.canMove` true)))))

(event `CheckForGameEnd`
  ;[1 1 1] Has Game Ended?
  (bind _returnvalue (`KismetSystemLibrary.K2_SetTimerDelegate` (delegate `EndTick`) 0.1 true))
  (set `self.GameEndTimer` _returnvalue))

(event `AddCheckpoint`
  (params (CheckpointNumber :type Integer))
  (bind _checkpointui (`self.CheckpointUI`))
  (bind _currentcheckpoint (`self.CurrentCheckpoint`))
  (bind _output (`|GetArrayItem` (`/Game/Blueprints/CheckpointManager.CheckpointArray` (`self.CheckpointManager`)) (- _currentcheckpoint 1)))
  ;[1 1 1] Checkpoints
  (if (== CheckpointNumber (+ _currentcheckpoint 1))
    (set `self.CurrentCheckpoint` CheckpointNumber)
    (`/Engine/EditorBlueprintResources/StandardMacros.IsValid` _checkpointui
      (:`Is Valid`
        (`TextBlock.SetText` (`/Game/UI/CheckpointCounter_UI.TextBlock_1` _checkpointui) (`KismetTextLibrary.Conv_IntToText` (`self.CurrentCheckpoint`)))))
    (elif (not (<= CheckpointNumber _currentcheckpoint))
      (`/Engine/EditorBlueprintResources/StandardMacros.IsValid` _output
        (:`Is Valid`
          (`self.K2_SetActorLocation` (`self.K2_GetActorLocation` _output)))))))

(event `InputAction|CameraFlip`
  (params (Key :type "Key Structure"))
  (bind _springarm (`self.SpringArm`))
  ;[1 1 1] ReverseCam
  (:`Pressed`
    (`SceneComponent.K2_SetRelativeRotation` _springarm (struct :`Yaw` 180.0) false false))
  (:`Released`
    (`SceneComponent.K2_SetRelativeRotation` :`self` _springarm)))

(event `EndTick`
  ;[1 1 1] Has Game Ended?
  (if (`/Game/Blueprints/GameModes/Boat_GM.hasGameEnded` (`self.As Boat GM`))
    (set `self.canBeFiredL` false)
    (set `self.canBeFiredR` false)
    (set `self.canJump` false)
    (set `self.canMove` false)))

(event `AutoMove`
  ;[1 1 1] Auto Move
  (bind _returnvalue (`KismetSystemLibrary.K2_SetTimerDelegate` (delegate `MoveTimer`) 0.1 true))
  (set `self.MoveHandle` _returnvalue))

(event `InputAxis|MoveForward`
  (params (AxisValue :type "Float (single-precision)"))
  ;[1 1 1] Movement
  (set `self.Axis Value` AxisValue)
  (if (`self.canMove`)
    (`PrimitiveComponent.AddForce` (* (* (`self.GetActorForwardVector`) (`self.ForwardSpeed`)) AxisValue) "None" true)))

(event `InputAction|Jump`
  (params (Key :type "Key Structure"))
  ;[1 1 1] Movement
  (:`Pressed`
    (if (`self.canJump`)
      (`PrimitiveComponent.AddForce` (* (`self.GetActorUpVector`) (`self.JumpStrength`)) "None" true)
      (set `self.canJump` false)
      (`KismetSystemLibrary.Delay` (`self.JumpDelay`))
      (set `self.canJump` true))))

(event `MoveTimer`
  ;[1 1 1] Auto Move
  (if (== (`self.Axis Value`) 0.0)
    (`PrimitiveComponent.AddForce` (* (`self.GetActorForwardVector`) 7000.0) "None" true)))

(event `InputAxis|MoveRight`
  (params (AxisValue :type "Float (single-precision)"))
  ;[1 1 1] Movement
  (if (`self.canMove`)
    (bind _returnvalue (`PrimitiveComponent.GetPhysicsLinearVelocity` "None"))
    (`PrimitiveComponent.AddTorqueInDegrees` (`KismetMathLibrary.MakeVector` 0.0 0.0 (* (`KismetMathLibrary.SelectFloat` 1.0 -1.0 (> (`KismetMathLibrary.Dot_VectorVector` _returnvalue (`self.GetActorForwardVector`)) 0.0)) (* AxisValue (`self.TurningSpeed`)))) "None" true)))

(event `InputAction|FireR`
  (params (Key :type "Key Structure"))
  (bind _rcannon (`self.RCannon`))
  (bind (_returnvalue_location _returnvalue_rotation) (`KismetMathLibrary.BreakTransform` (`SceneComponent.K2_GetComponentToWorld` _rcannon)))
  ;[1 1 1] Fire
  (:`Pressed`
    (if (`self.canBeFiredR`)
      (`PrimitiveComponent.AddImpulseAtLocation` (* (`SceneComponent.GetForwardVector` _rcannon) (`self.Kickback`)) (`SceneComponent.K2_GetComponentLocation` _rcannon))
      (`|SpawnActorFromClass` (`self.Projectile`) (`KismetMathLibrary.MakeTransform` _returnvalue_location _returnvalue_rotation (`self.ProjectileSize`)) "AdjustIfPossibleButAlwaysSpawn" "OverrideRootScale" null null)
      (set `self.canBeFiredR` false)
      (`self.CoolDownR`))))

(event `CoolDownR`
  ;[1 1 1] Cooldown Switch R
  (switch `/Game/Blueprints/BoatPawns/Cooldown_Enum` (`self.FireDelay`)
    (:`NewEnumerator0`
      (bind (_direction _percentage) (`Timeline|RCooldown1` :!via `PlayFromStart`)
        (:`Update`
          (`/Game/UI/ProjectileWidget.UpdateUI` (`self.RProjectileUI`) _percentage))
        (:`Finished`
          (set `self.canBeFiredR` true))))
    (:`NewEnumerator1`
      (bind (_direction_2 _percentage_2) (`Timeline|RCoolDown2` :!via `PlayFromStart`)
        (:`Update`
          (`/Game/UI/ProjectileWidget.UpdateUI` (`self.RProjectileUI`) _percentage_2))
        (:`Finished`
          (set `self.canBeFiredR` true))))
    (:`NewEnumerator2`
      (bind (_direction_3 _percentage_3) (`Timeline|RCoolDown5` :!via `PlayFromStart`)
        (:`Update`
          (`/Game/UI/ProjectileWidget.UpdateUI` (`self.RProjectileUI`) _percentage_3))
        (:`Finished`
          (set `self.canBeFiredR` true))))))

(event `InputAction|FireL`
  (params (Key :type "Key Structure"))
  (bind _lcannon (`self.LCannon`))
  (bind (_returnvalue_location _returnvalue_rotation) (`KismetMathLibrary.BreakTransform` (`SceneComponent.K2_GetComponentToWorld` _lcannon)))
  ;[1 1 1] Fire
  (:`Pressed`
    (if (`self.canBeFiredL`)
      (`PrimitiveComponent.AddImpulseAtLocation` (* (`SceneComponent.GetForwardVector` _lcannon) (`self.Kickback`)) (`SceneComponent.K2_GetComponentLocation` _lcannon))
      (`|SpawnActorFromClass` (`self.Projectile`) (`KismetMathLibrary.MakeTransform` _returnvalue_location _returnvalue_rotation (`self.ProjectileSize`)) "AdjustIfPossibleButAlwaysSpawn" "OverrideRootScale" null null)
      (set `self.canBeFiredL` false)
      (`self.CoolDownL`))))

(event `self.StaticMesh.OnComponentHit`
  (params (HitComponent :type "PrimitiveComponent Object Reference") (OtherActor :type "Actor Object Reference") (OtherComp :type "PrimitiveComponent Object Reference") (NormalImpulse :type "Vector Structure") (Hit :type "HitResult Structure (by ref)"))
  (bind (_bblockinghit _binitialoverlap _time _distance _location _impactpoint _normal _impactnormal _physmat _hitactor) (`GameplayStatics.BreakHitResult` Hit))
  (bind _damageduration (`self.DamageDuration`))
  ;[1 1 1] Damage
  (bind _asbase_projectile (castclass `/Game/Blueprints/Projectiles/Base_Projectile` (`GameplayStatics.GetObjectClass` _hitactor)))
  (bind _returnvalue (`GameplayStatics.GetActorOfClass` _asbase_projectile))
  (`PrimitiveComponent.AddImpulseAtLocation` (* (`self.GetActorForwardVector` _returnvalue) (`/Game/Blueprints/Projectiles/Base_Projectile.ImpactForce` _returnvalue)) _impactpoint)
  (`self.K2_DestroyActor` _returnvalue)
  (`self.DamageFlash`)
  (`|ExecutionSequence`
    (:`then_0`
      (bind _asboat_1_pc (cast `/Game/Blueprints/Boat1_PC` (`self.GetController` self))
        (:`then`
          (`self.DisableInput` _asboat_1_pc)
          (`KismetSystemLibrary.Delay` _damageduration)
          (`self.EnableInput` _asboat_1_pc))
        (:`CastFailed`
          (if (not (`self.isPossessed`))
            (`self.Damage`)
            (`KismetSystemLibrary.Delay` _damageduration)
            (`self.Continue`)))))
    (:`then_1`
      (`KismetSystemLibrary.Delay` (`self.DamageDuration`))
      (`KismetSystemLibrary.K2_ClearAndInvalidateTimerHandle` (`self.FlashTimerHandle`))
      (`SceneComponent.SetVisibility` true))))

(event `DamageFlash`
  ;[1 1 1] Flash
  (bind _returnvalue (`KismetSystemLibrary.K2_SetTimerDelegate` (delegate `Flash`) 0.1 true))
  (set `self.FlashTimerHandle` _returnvalue))

(event `CoolDownL`
  ;[1 1 1] CooldownL
  (switch `/Game/Blueprints/BoatPawns/Cooldown_Enum` (`self.FireDelay`)
    (:`NewEnumerator0`
      (bind (_direction _percentage) (`Timeline|LCooldown1` :!via `PlayFromStart`)
        (:`Update`
          (`/Game/UI/ProjectileWidget.UpdateUI` (`self.LProjectileUI`) _percentage))
        (:`Finished`
          (set `self.canBeFiredL` true))))
    (:`NewEnumerator1`
      (bind (_direction_2 _percentage_2) (`Timeline|LCoolDown2` :!via `PlayFromStart`)
        (:`Update`
          (`/Game/UI/ProjectileWidget.UpdateUI` (`self.LProjectileUI`) _percentage_2))
        (:`Finished`
          (set `self.canBeFiredL` true))))
    (:`NewEnumerator2`
      (bind (_direction_3 _percentage_3) (`Timeline|LCoolDown5` :!via `PlayFromStart`)
        (:`Update`
          (`/Game/UI/ProjectileWidget.UpdateUI` (`self.LProjectileUI`) _percentage_3))
        (:`Finished`
          (set `self.canBeFiredL` true))))))

(event `Flash`
  ;[1 1 1] Flash
  (`SceneComponent.ToggleVisibility` false))

(fn `InitHoverComponents`
  (`/Game/Blueprints/HoverComponent_SC.InitComponent` (`self.HoverComponent_SC`) null)
  (`/Game/Blueprints/HoverComponent_SC.InitComponent` (`self.HoverComponent_SC1`) null)
  (`/Game/Blueprints/HoverComponent_SC.InitComponent` (`self.HoverComponent_SC2`) null)
  (`/Game/Blueprints/HoverComponent_SC.InitComponent` (`self.HoverComponent_SC3`) null))

(fn `SetProjectileWidgets`
  (bind _asprojectile_widget (cast `/Game/UI/ProjectileWidget` (`WidgetComponent.GetUserWidgetObject` (`self.RWidget`))))
  (set `self.RProjectileUI` _asprojectile_widget)
  (bind _asprojectile_widget_2 (cast `/Game/UI/ProjectileWidget` (`WidgetComponent.GetUserWidgetObject` (`self.LWidget`))))
  (set `self.LProjectileUI` _asprojectile_widget_2))

(fn `UserConstructionScript`
  (bind (_impactforce _knockback) (defaults `Object` (`self.Projectile`)))
  (bind _asboat_gm (cast `/Game/Blueprints/GameModes/Boat_GM` (`GameplayStatics.GetGameMode`)))
  (set `self.As Boat GM` _asboat_gm)
  (set `self.ImpactForce` _impactforce)
  (set `self.Kickback` _knockback)
  (bind _returnvalue (`GameplayStatics.GetActorOfClass` "/Game/Blueprints/CheckpointManager.CheckpointManager_C"))
  (set `self.CheckpointManager` _returnvalue)
  (bind _returnvalue_2 (`GameplayStatics.GetActorOfClass` "/Game/Blueprints/Spline_BP.Spline_BP_C"))
  (set `self.splineReference` _returnvalue_2))