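; Ramp Blueprint that temporarily changes a boat's forward speed while the boat is inside its Box trigger.
; On overlap begin, it stores the first BaseBoat_Pawn and its original ForwardSpeed, then scales that speed by Multiplier.
; When that same boat leaves, it restores the saved speed and clears the reference.
; It tracks only one boat at a time, so others entering meanwhile are unaffected.
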(event `self.Box.OnComponentBeginOverlap`
  (params (OverlappedComponent :type "PrimitiveComponent Object Reference") (OtherActor :type "Actor Object Reference") (OtherComp :type "PrimitiveComponent Object Reference") (OtherBodyIndex :type Integer) (bFromSweep :type Boolean) (SweepResult :type "HitResult Structure (by ref)"))
  (bind _asbase_boat_pawn (cast `/Game/Blueprints/BoatPawns/BaseBoat_Pawn` OtherActor))
  (`/Engine/EditorBlueprintResources/StandardMacros.IsValid` (`self.As Base Boat Pawn`)
    (:`Is Not Valid`
      (bind _output_get (set `self.As Base Boat Pawn` _asbase_boat_pawn))
      (bind _output_get_2 (set `self.InitialSpeed` (`/Game/Blueprints/BoatPawns/BaseBoat_Pawn.ForwardSpeed` _output_get)))
      (set `/Game/Blueprints/BoatPawns/BaseBoat_Pawn.ForwardSpeed` (* _output_get_2 (`self.Multiplier`)) _output_get))))

(event `self.Box.OnComponentEndOverlap`
  (params (OverlappedComponent :type "PrimitiveComponent Object Reference") (OtherActor :type "Actor Object Reference") (OtherComp :type "PrimitiveComponent Object Reference") (OtherBodyIndex :type Integer))
  (bind _as_base_boat_pawn (`self.As Base Boat Pawn`))
  (bind _asbase_boat_pawn (cast `/Game/Blueprints/BoatPawns/BaseBoat_Pawn` OtherActor))
  (if (== _asbase_boat_pawn _as_base_boat_pawn)
    (set `/Game/Blueprints/BoatPawns/BaseBoat_Pawn.ForwardSpeed` (`self.InitialSpeed`) _as_base_boat_pawn)
    (set `self.As Base Boat Pawn` null)))

(fn `UserConstructionScript`)