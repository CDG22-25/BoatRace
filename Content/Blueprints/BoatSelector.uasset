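; BoatSelector is a boat selection Blueprint that cycles through four boats: Construction, Bath, Trash and Bird.
; Its UpdateBoat event steps ShipIndex forward or backward through the UpdateIndex function, which wraps around at both ends.
; The new index drives Select nodes that swap the displayed static mesh and set BoatType to the matching pawn.
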(event `UpdateBoat`
  (params (`next?` :type Boolean))
  (bind _oudex (`self.UpdateIndex` (`self.ShipIndex`) `next?`))
  (set `self.ShipIndex` _oudex)
  (`StaticMeshComponent.SetStaticMesh` (`self.StaticMesh`) (select `int` (`self.ShipIndex`) :`0` "/Game/Imports/Models/DiggerBoat/ConstructionboatUnwrap.ConstructionboatUnwrap" :`1` "/Game/Imports/Models/BathBoat/BathBoat.BathBoat" :`2` "/Game/Imports/Models/TrashBoat/TrashBoat_Moving.TrashBoat_Moving" :`3` "/Game/Imports/Models/BirdBoat/BirdBoatMoving.BirdBoatMoving" :!type "StaticMesh Object Reference"))
  (set `self.BoatType` (select `int` (`self.ShipIndex`) :`0` "/Game/Blueprints/BoatPawns/Construction_Pawn.Construction_Pawn_C" :`1` "/Game/Blueprints/BoatPawns/BathBoat_Pawn.BathBoat_Pawn_C" :`2` "/Game/Blueprints/BoatPawns/TrashBoat_Pawn.TrashBoat_Pawn_C" :`3` "/Game/Blueprints/BoatPawns/BirdBoat_Pawn.BirdBoat_Pawn_C" :!type "/Game/Blueprints/BoatPawns/BaseBoat_Pawn Class Reference")))

(fn `UpdateIndex`
  (params (Index :type Integer) (`next?` :type Boolean))
  (returns (oudex :type Integer))
  (locals (Value :type Integer))
  (if `next?`
    ;[1 1 1] Positive
    (bind _result (`/Engine/EditorBlueprintResources/StandardMacros.IncrementInt` Index)
      (:`  `
        (if (>= _result 4)
          (set `local.Value` 0)
          (else
            (set `local.Value` _result)))))
    (else
      ;[1 1 1] Negative
      (bind _result_2 (`/Engine/EditorBlueprintResources/StandardMacros.DecrementInt` Index)
        (:`  `
          (if (< _result_2 0)
            (set `local.Value` 3)
            (else
              (set `local.Value` _result_2)))))))
  (return (`local.Value`)))

(fn `UserConstructionScript`)