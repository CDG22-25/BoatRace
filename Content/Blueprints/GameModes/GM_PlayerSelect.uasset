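; Game mode for the local multiplayer player-select screen, where players choose boats and ready up before a match.
; On BeginPlay it recreates local players from the playerCount option, binds their PlayerSelect_PC ready events and shows the selection UI.
; Once players one and two are ready (two is automatic in solo), it saves boats to CustomBoatGameInstance and opens its chosen level and game mode.
; Player three and four handling is mostly disconnected.
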(event `self.ReceiveBeginPlay`
  ;[1 1 1] Begin Play
  (`self.Init`))

(event `Init`
  (bind _returnvalue (`GameplayStatics.GetIntOption` (`self.OptionsString`) "playerCount" 1))
  ;[1 1 1] Init
  (`WidgetBlueprintLibrary.SetInputMode_GameOnly` (`GameplayStatics.GetPlayerController` 0))
  (`self.RemovePlayers`)
  (`self.SetUpControllers` _returnvalue)
  (bind _returnvalue_2 (`|CreateWidget` "/Game/UI/Selection_UI.Selection_UI_C"))
  (bind _output_get (set `self.SelectionUI` _returnvalue_2))
  (`UserWidget.AddToViewport` _output_get 0)
  (`self.CorrectPlayers` _returnvalue))

(event `ReadyUp`
  (params (Player :type "/Game/Blueprints/PlayerSelect_PC Object Reference") (`Boat Selection` :type "/Game/Blueprints/BoatPawns/BaseBoat_Pawn Class Reference"))
  (bind _returnvalue (`GameplayStatics.GetPlayerControllerID` Player))
  ;[1 1 1] Ready Up
  (`/Game/UI/Selection_UI.DisplayReady` (`self.SelectionUI`) _returnvalue)
  (switch `int` _returnvalue
    (:`0`
      (set `self.Player1Boat` `Boat Selection`)
      (set `self.Player1Ready` true))
    (:`1`
      (set `self.Player2Boat` `Boat Selection`)
      (set `self.Player2Ready` true)))
  (if (and (`self.Player1Ready`) (`self.Player2Ready`) true true)
    (`/Game/Blueprints/CustomBoatGameInstance.SetPlayerSlections` (cast `/Game/Blueprints/CustomBoatGameInstance` (`GameplayStatics.GetGameInstance`) :!pure true) (`self.Player1Boat`) (`self.Player2Boat`))
    (`self.StartGame`)))

(event `UnReady`
  (params (Player :type "/Game/Blueprints/PlayerSelect_PC Object Reference"))
  (bind _returnvalue (`GameplayStatics.GetPlayerControllerID` Player))
  ;[1 1 1] Ready Up
  (`/Game/UI/Selection_UI.UnReady` (`self.SelectionUI`) _returnvalue)
  (switch `int` _returnvalue
    (:`0`
      (set `self.Player1Ready` false))
    (:`1`
      (set `self.Player2Ready` false))))

(event `StartGame`
  (bind _ascustom_boat_game_instance (cast `/Game/Blueprints/CustomBoatGameInstance` (`GameplayStatics.GetGameInstance`) :!pure true))
  ;[1 1 1] Start Game
  (`GameplayStatics.OpenLevel` (`/Game/Blueprints/CustomBoatGameInstance.Level Name` _ascustom_boat_game_instance) true (`KismetStringLibrary.Concat_StrStr` "game=" (`/Game/Blueprints/CustomBoatGameInstance.Game Mode Alias` _ascustom_boat_game_instance) "?playerCount=" (`KismetStringLibrary.Conv_IntToString` (`/Game/Blueprints/CustomBoatGameInstance.PlayerCount` _ascustom_boat_game_instance)))))

(event `self.K2_PostLogin`
  (params (NewPlayer :type "PlayerController Object Reference"))
  (`KismetArrayLibrary.Array_Add` (`self.PlayerControllers`) NewPlayer))

(event `self.K2_OnLogout`
  (params (ExitingController :type "Controller Object Reference"))
  (bind _asplayer_controller (cast `PlayerController` ExitingController))
  (`KismetArrayLibrary.Array_RemoveItem` (`self.PlayerControllers`) _asplayer_controller))

(fn `CorrectPlayers`
  (params (NumberOfPlayers :type Integer))
  (switch `int` NumberOfPlayers
    (:`1`
      (set `self.Player2Ready` true))))

(fn `RemovePlayers`
  (for _index (range 4)
    (bind _returnvalue (`GameplayStatics.GetPlayerController` _index))
    (`/Engine/EditorBlueprintResources/StandardMacros.IsValid` _returnvalue
      (:`Is Valid`
        (`GameplayStatics.RemovePlayer` _returnvalue true)))))

(fn `SetUpControllers`
  (params (NumberOfPlayers :type Integer))
  (for _index (range NumberOfPlayers)
    (bind _returnvalue (`GameplayStatics.CreatePlayer` _index))
    (bind _asplayer_select_pc (cast `/Game/Blueprints/PlayerSelect_PC` _returnvalue))
    (add `/Game/Blueprints/PlayerSelect_PC.ReadyUp` _asplayer_select_pc (`|CreateDelegate` :!event `ReadyUp`))
    (add `/Game/Blueprints/PlayerSelect_PC.UnReady` _asplayer_select_pc (`|CreateDelegate` :!event `UnReady`))
    (switch `int` NumberOfPlayers
      (:`2`
        (set `self.Player3Ready` true)
        (set `self.Player4Ready` true))
      (:`3`
        (set `self.Player4Ready` true)))))

(fn `UserConstructionScript`)