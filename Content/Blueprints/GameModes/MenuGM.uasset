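; Main menu game mode for what appears to be a local multiplayer boat game.
; On BeginPlay it resets local players to a single new one, clears the game instance's player selections and shows the Start_Menu_Final widget with UI-only input.
; PlayerSelect stores the player count in the game instance and opens the PlayerSelection level.
; StartGame opens a given level, passing the game mode alias and player count as URL options.
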(event `self.ReceiveBeginPlay`
  (bind _returnvalue (`GameplayStatics.GetPlayerController` 0))
  ;[1 1 1] Begin
  (`self.RemovePlayers`)
  (bind _output_get (set `self.As Custom Game Instance` (cast `/Game/Blueprints/CustomBoatGameInstance` (`GameplayStatics.GetGameInstance`) :!pure true)))
  (`KismetArrayLibrary.Array_Clear` (`/Game/Blueprints/CustomBoatGameInstance.PlayerSelections` _output_get))
  (bind _returnvalue_2 (`|CreateWidget` "/Game/EdwardsFile/EdwardsFileUpdate/UI/Start_Menu_Final.Start_Menu_Final_C" (`GameplayStatics.GetPlayerController` 0)))
  (bind _output_get_2 (set `self.MenuNew` _returnvalue_2))
  (`UserWidget.AddToViewport` _output_get_2 0)
  (`WidgetBlueprintLibrary.SetInputMode_UIOnlyEx` _returnvalue (`self.MenuUI`))
  (set `PlayerController.bShowMouseCursor` true _returnvalue))

(event `StartGame`
  (params (NumberOfPlayers :type Integer) (LevelName :type Name) (GameModeAlias :type String))
  ;[1 1 1] StartGame
  (`GameplayStatics.OpenLevel` LevelName true (`KismetStringLibrary.Concat_StrStr` "game=" GameModeAlias "?playerCount=" (`KismetStringLibrary.Conv_IntToString` NumberOfPlayers))))

(event `PlayerSelect`
  (params (Players :type Integer))
  ;[1 1 1] PlayerSelect
  (set `/Game/Blueprints/CustomBoatGameInstance.PlayerCount` Players (`self.As Custom Game Instance`))
  (`GameplayStatics.OpenLevel` "PlayerSelection" true (`KismetStringLibrary.Concat_StrStr` "?playerCount=" (`KismetStringLibrary.Conv_IntToString` Players))))

(fn `RemovePlayers`
  (for _index (range 4)
    (bind _returnvalue (`GameplayStatics.GetPlayerController` _index))
    (`/Engine/EditorBlueprintResources/StandardMacros.IsValid` _returnvalue
      (:`Is Valid`
        (`GameplayStatics.RemovePlayer` _returnvalue true)
        (`KismetSystemLibrary.PrintString` "Players Removed"))))
  (bind _returnvalue_2 (`GameplayStatics.CreatePlayer` 0))
  (`KismetSystemLibrary.PrintString` (`KismetStringLibrary.Concat_StrStr` (`KismetSystemLibrary.GetDisplayName` _returnvalue_2) " created")))

(fn `UserConstructionScript`)