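; Physics-driven boat pawn that hovers on four HoverComponents, auto-accelerates forward, and fires left and right cannons.
; Input adds forces and torque for thrust, steering and jumping, while cooldown-limited shots apply recoil from the Projectile class defaults.
; Projectile hits shove and flash the boat and briefly disable Boat1_PC input, using GetActorOfClass rather than the hit actor.
; Tick temporarily disables input when the boat flies too high.
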(event `self.ReceiveTick`
  (params (DeltaSeconds :type "Float (single-precision)"))
  (bind (_returnvalue_x _returnvalue_y _returnvalue_z) (`KismetMathLibrary.BreakVector` (`self.K2_GetActorLocation`)))
  ;[1 1 1] Flying Fix
  (if (> _returnvalue_z 300.0)
    (`self.DisableInput` null)
    (`KismetSystemLibrary.Delay` 2.0)
    (`self.EnableInput` null)))

(event `self.ReceiveBeginPlay`
  (bind _staticmesh (`self.StaticMesh`))
  (bind (_impactforce _knockback) (defaults `Object` (`self.Projectile`)))
  ;[1 1 1] Begin Play
  (set `self.ImpactForce` _impactforce)
  (set `self.Kickback` _knockback)
  (`/Game/Blueprints/HoverComponent_SC.InitComponent` (`self.HoverComponent_SC`) _staticmesh)
  (`/Game/Blueprints/HoverComponent_SC.InitComponent` (`self.HoverComponent_SC1`) _staticmesh)
  (`/Game/Blueprints/HoverComponent_SC.InitComponent` (`self.HoverComponent_SC2`) _staticmesh)
  (`/Game/Blueprints/HoverComponent_SC.InitComponent` (`self.HoverComponent_SC3`) _staticmesh)
  (`self.AutoMove`))

(event `AutoMove`
  ;[1 1 1] Auto Move
  (bind _returnvalue (`KismetSystemLibrary.K2_SetTimerDelegate` (delegate `MoveTimer`) 0.1 true))
  (set `self.MoveHandle` _returnvalue))

(event `InputAxis|MoveForward`
  (params (AxisValue :type "Float (single-precision)"))
  ;[1 1 1] Movement
  (if (`self.canMove`)
    (`PrimitiveComponent.AddForce` (`self.StaticMesh`) (* (* (`self.GetActorForwardVector`) (`self.ForwardSpeed`)) AxisValue) "None" true)))

(event `InputAction|Jump`
  (params (Key :type "Key Structure"))
  ;[1 1 1] Movement
  (:`Pressed`
    (if (`self.canJump`)
      (`PrimitiveComponent.AddForce` (`self.StaticMesh`) (* (`self.GetActorUpVector`) (`self.JumpStrength`)) "None" true)
      (set `self.canJump` false)
      (`KismetSystemLibrary.Delay` (`self.JumpDelay`))
      (set `self.canJump` true))))

(event `MoveTimer`
  ;[1 1 1] Auto Move
  (`PrimitiveComponent.AddForce` (`self.StaticMesh`) (* (`self.GetActorForwardVector`) 7000.0) "None" true))

(event `InputAxis|MoveRight`
  (params (AxisValue :type "Float (single-precision)"))
  ;[1 1 1] Movement
  (if (`self.canMove`)
    (bind _returnvalue (`PrimitiveComponent.GetPhysicsLinearVelocity` (`self.StaticMesh`) "None"))
    (`PrimitiveComponent.AddTorqueInDegrees` (`self.StaticMesh`) (`KismetMathLibrary.MakeVector` 0.0 0.0 (* (`KismetMathLibrary.SelectFloat` 1.0 -1.0 (> (`KismetMathLibrary.Dot_VectorVector` _returnvalue (`self.GetActorForwardVector`)) 0.0)) (* AxisValue (`self.TurningSpeed`)))) "None" true)))

(event `InputAction|FireR`
  (params (Key :type "Key Structure"))
  (bind _rcannon (`self.RCannon`))
  (bind (_returnvalue_location _returnvalue_rotation) (`KismetMathLibrary.BreakTransform` (`SceneComponent.K2_GetComponentToWorld` _rcannon)))
  ;[1 1 1] Fire
  (:`Pressed`
    (if (`self.canBeFiredR`)
      (`PrimitiveComponent.AddImpulseAtLocation` (`self.StaticMesh`) (* (`SceneComponent.GetForwardVector` _rcannon) (`self.Kickback`)) (`SceneComponent.K2_GetComponentLocation` _rcannon) "None")
      (`|SpawnActorFromClass` (`self.Projectile`) (`KismetMathLibrary.MakeTransform` _returnvalue_location _returnvalue_rotation (`self.ProjectileSize`)) "AdjustIfPossibleButAlwaysSpawn" "OverrideRootScale" null null)
      (set `self.canBeFiredR` false)
      (`KismetSystemLibrary.Delay` (`self.FireDelay`))
      (set `self.canBeFiredR` true))))

(event `InputAction|FireL`
  (params (Key :type "Key Structure"))
  (bind _lcannon (`self.LCannon`))
  (bind (_returnvalue_location _returnvalue_rotation) (`KismetMathLibrary.BreakTransform` (`SceneComponent.K2_GetComponentToWorld` _lcannon)))
  ;[1 1 1] Fire
  (:`Pressed`
    (if (`self.canBeFiredL`)
      (`PrimitiveComponent.AddImpulseAtLocation` (`self.StaticMesh`) (* (`SceneComponent.GetForwardVector` _lcannon) (`self.Kickback`)) (`SceneComponent.K2_GetComponentLocation` _lcannon) "None")
      (`|SpawnActorFromClass` (`self.Projectile`) (`KismetMathLibrary.MakeTransform` _returnvalue_location _returnvalue_rotation (`self.ProjectileSize`)) "AdjustIfPossibleButAlwaysSpawn" "OverrideRootScale" null null)
      (set `self.canBeFiredL` false)
      (`KismetSystemLibrary.Delay` (`self.FireDelay`))
      (set `self.canBeFiredL` true))))

(event `self.StaticMesh.OnComponentHit`
  (params (HitComponent :type "PrimitiveComponent Object Reference") (OtherActor :type "Actor Object Reference") (OtherComp :type "PrimitiveComponent Object Reference") (NormalImpulse :type "Vector Structure") (Hit :type "HitResult Structure (by ref)"))
  (bind (_bblockinghit _binitialoverlap _time _distance _location _impactpoint _normal _impactnormal _physmat _hitactor) (`GameplayStatics.BreakHitResult` Hit))
  ;[1 1 1] Damage
  (bind _asprojectile (castclass `/Game/Blueprints/Projectile` (`GameplayStatics.GetObjectClass` _hitactor)))
  (bind _returnvalue (`GameplayStatics.GetActorOfClass` _asprojectile))
  (`PrimitiveComponent.AddImpulseAtLocation` (`self.StaticMesh`) (* (`self.GetActorForwardVector` _returnvalue) (`/Game/Blueprints/Projectile.ImpactForce` _returnvalue)) _impactpoint "None")
  (`self.K2_DestroyActor` _returnvalue)
  (`self.DamageFlash`)
  (`KismetSystemLibrary.PrintString` "Hit")
  (`|ExecutionSequence`
    (:`then_0`
      (bind _asboat_1_pc (cast `/Game/Blueprints/Boat1_PC` (`self.GetController` self)))
      (`self.DisableInput` _asboat_1_pc)
      (`KismetSystemLibrary.Delay` (`self.DamageDuration`))
      (`self.EnableInput` _asboat_1_pc))
    (:`then_1`
      (`KismetSystemLibrary.Delay` (`self.DamageDuration`))
      (`KismetSystemLibrary.K2_ClearAndInvalidateTimerHandle` (`self.FlashTimerHandle`))
      (`SceneComponent.SetVisibility` (`self.StaticMesh`) true false))))

(event `DamageFlash`
  ;[1 1 1] Flash
  (bind _returnvalue (`KismetSystemLibrary.K2_SetTimerDelegate` (delegate `Flash`) 0.1 true))
  (set `self.FlashTimerHandle` _returnvalue))

(event `Flash`
  ;[1 1 1] Flash
  (`SceneComponent.ToggleVisibility` (`self.StaticMesh`) false))

(fn `UserConstructionScript`)