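; Trial manager for a boat time trial, tracking lap times and checkpoint progress for the trial UI.
; Init binds to every Checkpoint and the Finish_BP, and game state changes start or clear a looping 0.01-second timer that increments the count.
; Checkpoint hits read the boat's current lap and update the UI.
; Finish crossings post lap times, resetting after laps 1 and 2; all three laps write to Lap1Time.
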(event `Init`
  ;[1 1 1] Init
  (bind _asgm_trial (cast `/Game/Blueprints/GameModes/GM_Trial` (`GameplayStatics.GetGameMode`)))
  (set `self.GameMode` _asgm_trial)
  (`self.GetCheckpoints`)
  (bind _returnvalue (`GameplayStatics.GetActorOfClass` "/Game/Blueprints/Finish_BP.Finish_BP_C"))
  (add `/Game/Blueprints/Finish_BP.FinishLine` _returnvalue (`|CreateDelegate` :!event `FinishLine`)))

(event `StartTimer`
  ;[1 1 1] Timer
  (bind _returnvalue (`KismetSystemLibrary.K2_SetTimerDelegate` (delegate `TimerTick`) 0.01 true))
  (set `self.Timer Handle` _returnvalue))

(event `TimerTick`
  ;[1 1 1] Timer
  (set `self.TimerCount` (+ (`self.TimerCount`) 0.01)))

(event `/Game/Blueprints/I_GameState.GameStateChanged`
  (params (newGameState :type "/Game/Blueprints/E_GameState Enum" :default "NewEnumerator0"))
  ;[1 1 1] Game State Changed
  (switch `/Game/Blueprints/E_GameState` newGameState
    (:`NewEnumerator2`
      (`self.StartTimer`))
    (:`NewEnumerator3`
      (`KismetSystemLibrary.K2_ClearAndInvalidateTimerHandle` (`self.Timer Handle`)))))

(event `FinishLine`
  (bind _timercount (`self.TimerCount`))
  (switch `int` (`self.Lap`)
    (:`1`
      (set `self.Lap1Time` _timercount)
      (`/Game/UI/Trial_UI.Set Lap Time` (`/Game/Blueprints/GameModes/GM_Trial.Trial UI` (`self.GameMode`)) (`self.Lap`) (`self.TimerCount`) :!label _label)
      (set `self.TimerCount` 0.0))
    (:`2`
      (set `self.Lap1Time` _timercount)
      (goto _label))
    (:`3`
      (set `self.Lap1Time` _timercount)
      (`/Game/UI/Trial_UI.Set Lap Time` (`/Game/Blueprints/GameModes/GM_Trial.Trial UI` (`self.GameMode`)) (`self.Lap`) (`self.TimerCount`)))))

(event `CheckpointHit`
  (params (`Checkpoint Number` :type Integer) (Player :type Integer))
  (bind _asbase_boat_pawn (cast `/Game/Blueprints/BoatPawns/BaseBoat_Pawn` (`Controller.K2_GetPawn` (`GameplayStatics.GetPlayerControllerFromID` Player))))
  (bind _currentlap (`/Game/Blueprints/BoatPawns/BaseBoat_Pawn.CurrentLap` _asbase_boat_pawn))
  (set `self.Lap` _currentlap)
  (`/Game/UI/Trial_UI.UpdateUI` (`/Game/Blueprints/GameModes/GM_Trial.Trial UI` (`self.GameMode`)) (`/Game/Blueprints/BoatPawns/BaseBoat_Pawn.CurrentCheckpoint` _asbase_boat_pawn) _currentlap))

(fn `GetCheckpoints`
  (bind _outactors (`GameplayStatics.GetAllActorsOfClass` "/Game/Blueprints/Checkpoint.Checkpoint_C"))
  (bind _output_get (set `self.Checkpoints` _outactors))
  (add `/Game/Blueprints/Checkpoint.CheckpointHit` _output_get (`|CreateDelegate` :!event `CheckpointHit`)))

(fn `UserConstructionScript`)