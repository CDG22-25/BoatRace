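; Spinner is a one-shot hazard actor that spins out any BaseBoat_Pawn overlapping it, other than its Parent boat, while it is active.
; On a hit it deactivates, hides its root component and starts a fast looping timer that disables the boat's movement and applies yaw torque to its mesh.
; A one-second timer then restores movement, clears the spin timer and destroys the actor.
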(event `self.ReceiveBeginPlay`
  (`parent.ReceiveBeginPlay`))

(event `self.ReceiveActorBeginOverlap`
  (params (OtherActor :type "Actor Object Reference"))
  (if (`self.Active`)
    (bind _asbase_boat_pawn (cast `/Game/Blueprints/BoatPawns/BaseBoat_Pawn` OtherActor))
    (if (not (== _asbase_boat_pawn (`self.Parent`)))
      (`self.Spin` _asbase_boat_pawn)
      (set `self.Active` false)
      (`SceneComponent.SetVisibility` (`self.DefaultSceneRoot`) false false)
      (`KismetSystemLibrary.PrintString` "Spin"))))

(event `Spin`
  (params (Boat :type "/Game/Blueprints/BoatPawns/BaseBoat_Pawn Object Reference"))
  (bind _returnvalue (`KismetSystemLibrary.K2_SetTimerDelegate` (delegate `Spinning`) 0.03 true))
  (`KismetSystemLibrary.K2_SetTimerDelegate` (delegate `StopSpinning`) 1.0))

(event `Spinning`
  (set `/Game/Blueprints/BoatPawns/BaseBoat_Pawn.canMove` false (stale `Spin` Boat))
  (`PrimitiveComponent.AddTorqueInDegrees` (`/Game/Blueprints/BoatPawns/BaseBoat_Pawn.StaticMesh` (stale `Spin` Boat)) (0.0 0.0 5000.0) "None" true))

(event `StopSpinning`
  (set `/Game/Blueprints/BoatPawns/BaseBoat_Pawn.canMove` true (stale `Spin` Boat))
  (`KismetSystemLibrary.K2_PauseTimerHandle` (stale `Spin` _returnvalue))
  (`KismetSystemLibrary.K2_ClearAndInvalidateTimerHandle` (stale `Spin` _returnvalue))
  (`self.K2_DestroyActor`))

(fn `UserConstructionScript`)