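; Race manager that tracks players' checkpoint progress and refreshes the race UI.
; Init binds events on the level's Checkpoint_Manager and its checkpoints, then fires two debug events after a short delay.
; Checkpoint hits store the checkpoint number in a map keyed by player index plus one.
; Checkpoint updates pass that player's boat pawn's current checkpoint to GM_Race's UI.
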(event `Init`
  ;[1 1 1] Init
  (bind _returnvalue (`GameplayStatics.GetActorOfClass` "/Game/Blueprints/Checkpoint_Manager.Checkpoint_Manager_C"))
  (add `/Game/Blueprints/Checkpoint.CheckpointHit` (`/Game/Blueprints/Checkpoint_Manager.Checkpoints` _returnvalue) (`|CreateDelegate` :!event `CheckpointHit`))
  (add `/Game/Blueprints/Checkpoint_Manager.CheckpointUpdated` _returnvalue (`|CreateDelegate` :!event `CheckpointUpdated`))
  (`KismetSystemLibrary.Delay` 3.0)
  (`self.HitDebug`)
  (`self.UpdateDebug`))

(event `HitDebug`
  (`KismetSystemLibrary.PrintString` "HitDebug")
  ;[1 1 1] CheckpointHit
  (`BlueprintMapLibrary.Map_Add` (`self.PlayerCheckpointPositions`) (+ (stale `CheckpointHit` Player) 1) (stale `CheckpointHit` `Checkpoint Number`) :!label _label))

(event `CheckpointHit`
  (params (`Checkpoint Number` :type Integer) (Player :type Integer))
  ;[1 1 1] CheckpointHit
  (goto _label))

(event `CheckpointUpdated`
  (params (Player :type Integer))
  ;[1 1 1] CheckpointUpdated
  (bind _asgm_race (cast `/Game/Blueprints/GameModes/GM_Race` (`GameplayStatics.GetGameMode`) :!label _label_2))
  (bind _asbase_boat_pawn (cast `/Game/Blueprints/BoatPawns/BaseBoat_Pawn` (`Controller.K2_GetPawn` (`GameplayStatics.GetPlayerControllerFromID` Player))))
  (`/Game/UI/CheckpointCounter_UI.UpdateUI` (`/Game/Blueprints/GameModes/GM_Race.Race UI` _asgm_race) (`/Game/Blueprints/BoatPawns/BaseBoat_Pawn.CurrentCheckpoint` _asbase_boat_pawn)))

(event `UpdateDebug`
  ;[1 1 1] CheckpointUpdated
  (`KismetSystemLibrary.PrintString` "UpdateDebug")
  (goto _label_2))

(fn `UserConstructionScript`)