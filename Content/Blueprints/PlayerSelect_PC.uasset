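; Player controller for the boat selection screen, letting a player cycle boats, ready up and unready.
; It receives a Manager via InitManager, forwards left/right input to it, and stores the boat class passed to SetBoat.
; Start broadcasts ReadyUp with that boat, and UnReady broadcasts its event; CanSelect gates swapping and readying but is never cleared here.
; GetManager and GetBoat are non-functional stubs.
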(event `Init Manager`
  (params (Manager :type "/Game/Blueprints/SelectManager Object Reference"))
  (set `self.Manager` Manager)
  (set `self.canSelect` true))

(event `InputAction|SwapBoatLeft`
  (params (Key :type "Key Structure"))
  ;[1 1 1] Selection
  (:`Pressed`
    (if (`self.canSelect`)
      (`/Game/Blueprints/SelectManager.PrevBoat` (`self.Manager`) self))))

(event `InputAction|SwapBoatRight`
  (params (Key :type "Key Structure"))
  ;[1 1 1] Selection
  (:`Pressed`
    (if (`self.canSelect`)
      (`/Game/Blueprints/SelectManager.NextBoat` (`self.Manager`) self))))

(event `InputAction|Start`
  (params (Key :type "Key Structure"))
  ;[1 1 1] Ready
  (:`Pressed`
    (if (`self.canSelect`)
      (`self.ReadyUp` self (`self.BoatType`))
      (`KismetSystemLibrary.PrintString` "ReadyUp"))))

(event `/Game/Blueprints/I_Boat.SetBoat`
  (params (BoatClass :type "/Game/Blueprints/BoatPawns/BaseBoat_Pawn Class Reference"))
  ;[1 1 1] Set Boat
  (set `self.BoatType` BoatClass))

(event `InputAction|UnReady`
  (params (Key :type "Key Structure"))
  ;[1 1 1] UnReady
  (:`Pressed`
    (set `self.canSelect` true)
    (`self.UnReady` self)))

(fn `GetBoat`
  (returns (BoatClass :type "/Game/Blueprints/BoatPawns/BaseBoat_Pawn Class Reference"))
  (return null))

(fn `GetManager`)

(fn `UserConstructionScript`)